(event `self.OnVictory`
  (for _array_element (`self.PlayerArray`)
    (bind _asnet_player_state (cast `NetPlayerState` _array_element))
    (bind (_data_nickname _data_customizationdata _data_teamid) (break `SPlayerInfo` (`NetPlayerState.Data` _asnet_player_state)))
    (switch `EPlayerTeam` _data_teamid
      (:`TEAM_Blue`
        (bind _asbp_net_avatar (cast `/Game/Blueprints/BP_NetAvatar` (`PlayerState.PawnPrivate` _asnet_player_state) :!pure true))
        (`/Game/Blueprints/BP_NetAvatar.OnPlayerLost` _asbp_net_avatar))
      (:`TEAM_Red`
        (`/Game/Blueprints/BP_NetAvatar.OnPlayerWon` _asbp_net_avatar)))))

(event `self.OnRestart`
  (`Widget.RemoveFromParent` (`self.MessageWidget`)))

(event `self.NoTimeLeft`
  (for _array_element (`self.PlayerArray`)
    (bind _asnet_player_state (cast `NetPlayerState` _array_element))
    (bind (_data_nickname _data_customizationdata _data_teamid) (break `SPlayerInfo` (`NetPlayerState.Data` _asnet_player_state)))
    (switch `EPlayerTeam` _data_teamid
      (:`TEAM_Blue`
        (bind _asbp_net_avatar (cast `/Game/Blueprints/BP_NetAvatar` (`PlayerState.PawnPrivate` _asnet_player_state) :!pure true))
        (`/Game/Blueprints/BP_NetAvatar.OnPlayerWon` _asbp_net_avatar))
      (:`TEAM_Red`
        (`/Game/Blueprints/BP_NetAvatar.OnPlayerLost` _asbp_net_avatar))))
  (`self.ShowResultsScreen`))

(fn `ShowResultsScreen`
  (bind (_data_nickname _data_customizationdata _data_teamid) (break `SPlayerInfo` (`NetPlayerState.Data` (cast `NetPlayerState` (`Controller.PlayerState` (`GameplayStatics.GetPlayerController` 0)) :!pure true))))
  (bind _returnvalue (`self.GetPlayerStateByIndex` (`self.WinningPlayer`)))
  (bind _returnvalue_2 (`|CreateWidget` "/Game/Blueprints/UMG/W_GameResults.W_GameResults_C" null (select `bool` (`|EnumEquality` _data_teamid "TEAM_Blue") :`false` (`|FormatText` "{Name} WINS!" (`.Nickname` (break `SPlayerInfo` (`NetPlayerState.Data` _returnvalue)))) :`true` "YOU LOSE!")))
  (bind _output_get (set `self.MessageWidget` _returnvalue_2))
  (`UserWidget.AddToViewport` _output_get 0))

(fn `UserConstructionScript`)